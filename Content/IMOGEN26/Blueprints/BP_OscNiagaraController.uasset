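; Niagara controller actor that drives effect parameters from incoming OSC messages.
; It spawns a shared OSC server if none exists and binds to its messages once ready.
; Addresses matching data table row names set typed Niagara variables, with floats linearly remapped without clamping.
; Addresses prefixed with this instance's system ID set spawn rate, visibility and enabled state, activating or deactivating the component; debug printing is optional.
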(event Custom|OnOSCMessageReceived
  (params (Message :type OSC%20Message%20Structure%20%28by%20ref%29) (IPAddress :type String) (Port :type Integer))
  (bind _niagara (Variables|Default|GetNiagara))
  (bind _niagaracomponent (Variables|/Script/Niagara.NiagaraActor|GetNiagaraComponent _niagara))
  ;[0 0 0] Get incoming address, convert to the format we want
  (bind _returnvalue (Class|OSCManager|GetOSCMessageAddress Message))
  (bind _returnvalue_2 (Class|OSCManager|GetOSCAddressFullPath _returnvalue))
  (Utilities|FlowControl|Sequence
    (:then_0
      (|Logging _returnvalue_2
        (:Enabled
          _)
        (:Disabled
          _))
      ;[0 0 0] If row name matches OSC address, send to niagara right away
      (bind _returnvalue_3 (Utilities|GetDataTableRow (Variables|Default|GetOSCParameterLinks) (Utilities|String|StringToName _returnvalue_2))
        (:then
          (CallFunction|OSCMessagetoNiagaraParameter Message _returnvalue_3 _returnvalue_2))))
    (:then_1
      ;[0 0 0] Write System Params for ID
      (if (Utilities|String|StartsWith _returnvalue_2 (Variables|Default|GetSystemAddress))
        (bind _value (Class|OSCManager|GetFloat Message))
        (switch string (.RightS (Utilities|String|Split _returnvalue_2 "/" "IgnoreCase" "FromEnd"))
          (:spawnrate
            (Niagara|SetNiagaraVariable(Float) _niagaracomponent "SystemSpawnRateMultiplier" _value))
          (:visibility
            (Niagara|SetNiagaraVariable(Float) _niagaracomponent "SystemVisibility" _value))
          (:enabled
            (Class|NiagaraComponent|SetVariableBool _niagaracomponent "SystemEnabled" (> _value 0.0))
            (if (> _value 0.0)
              (Components|Activation|Activate _niagaracomponent false)
              (else
                (Components|Activation|Deactivate _niagaracomponent)))))))))

(event Custom|OnSharedServerReady
  (params (OSC%20Server%20Instance :type OSC%20Server%20Object%20Reference))
  (Development|PrintString "Shared OSC server is ready...")
  (Utilities|FlowControl|Sequence
    (:then_0
      (Utilities|IsValid OSC%20Server%20Instance
        (:Is%20Valid
          ;[0 0 0] Setup event
          (EventDispatchers|BindEventtoOnOscMessageReceived OSC%20Server%20Instance (delegate Custom|OnOSCMessageReceived)))
        (:Is%20Not%20Valid
          (Development|PrintString "Server was not valid..."))))
    (:then_1
      ;[0 0 0] Cache names
      (bind _outrownames (DataTable|GetDataTableRowNames (Variables|Default|GetOSCParameterLinks)))
      (Variables|Default|SetData%20Table%20Row%20Names _outrownames))))

(event EventBeginPlay
  (Utilities|FlowControl|Sequence
    (:then_0
      ;[0 0 0] Create shared server if it isn't
      (bind _returnvalue (Actor|GetActorOfClass "/Game/IMOGEN26/Blueprints/BP_SharedOscServer.BP_SharedOscServer_C"))
      (Utilities|IsValid _returnvalue
        (:Is%20Not%20Valid
          (Game|SpawnActorfromClass "/Game/IMOGEN26/Blueprints/BP_SharedOscServer.BP_SharedOscServer_C" (Math|Transform|MakeTransform "0, 0, 0") "Undefined" "MultiplyWithRoot" 0 0)
          (Development|PrintString "Auto-Created shared OSC server setup."))))
    (:then_1
      (Variables|Default|SetSystemAddress (Utilities|String|Append "/system/" (Utilities|String|ToString(Integer) (Variables|Default|GetSystem%20ID)))))))

(fn ConstructionScript)

(fn OSCMessagetoNiagaraParameter
  (params (OSC%20Message :type OSC%20Message%20Structure%20%28by%20ref%29) (OSC%20To%20Niagara%20Mapping :type S%20OSC%20to%20Niagara%20Mapping%20Structure) (OSC%20Address :type String))
  (bind (_niagaraparametername _enabled _valuetype _instart _inend _outstart _outend) (Utilities|Struct|BreakS_OSCToNiagaraMapping OSC%20To%20Niagara%20Mapping))
  (bind _niagara (Variables|Default|GetNiagara))
  (bind _returnvalue (Utilities|String|ToString(Name) _niagaraparametername))
  (bind _niagaracomponent (Variables|/Script/Niagara.NiagaraActor|GetNiagaraComponent _niagara))
  (if _enabled
    (Utilities|IsValid _niagaracomponent
      (:Is%20Valid
        (switch Utilities|FlowControl|Switch|SwitchonEParamType _valuetype
          (:NewEnumerator0
            ;[0 0 0] floats with remap
            (bind _value (Class|OSCManager|GetFloat OSC%20Message))
            (if (Variables|Default|GetPrint%20Matched%20OSC%20Messages)
              (|LogFloats _value OSC%20Address _returnvalue))
            (Niagara|SetNiagaraVariable(Float) _niagaracomponent _niagaraparametername (Math|Float|MapRangeUnclamped _value _instart _inend _outstart _outend)))
          (:NewEnumerator1
            ;[0 0 0] integers
            (bind _value_2 (Class|OSCManager|GetInt32 OSC%20Message))
            (if (Variables|Default|GetPrint%20Matched%20OSC%20Messages)
              (|LogInts OSC%20Address _value_2 _returnvalue))
            (Class|NiagaraComponent|SetVariableInt _niagaracomponent _niagaraparametername _value_2))
          (:NewEnumerator2
            ;[0 0 0] booleans
            (bind _value_3 (Class|OSCManager|GetBool OSC%20Message))
            (if (Variables|Default|GetPrint%20Matched%20OSC%20Messages)
              (|LogBools OSC%20Address _value_3 _returnvalue))
            (Class|NiagaraComponent|SetVariableBool _niagaracomponent _niagaraparametername _value_3)))))))