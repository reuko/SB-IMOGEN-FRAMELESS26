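; Camera controller actor that scrubs a Level Sequence from OSC messages, spawning a shared OSC server if none exists.
; Once the server is ready it listens for /camera/ addresses: Id selects a zero-based camera index, Position sets a target time offset by that index.
; Tick eases toward the target and jumps the sequence playhead there, so each camera index starts one second further along the timeline.
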(event Custom|OnOSCMessageReceived
  (params (Message :type OSC%20Message%20Structure%20%28by%20ref%29) (IPAddress :type String) (Port :type Integer))
  (Utilities|FlowControl|Sequence
    (:then_0
      ;[0 0 0] Get incoming address, convert to the format we want
      (bind _returnvalue (Class|OSCManager|GetOSCMessageAddress Message))
      (bind _returnvalue_2 (Class|OSCManager|GetOSCAddressFullPath _returnvalue)))
    (:then_1
      ;[0 0 0] Do camera if assigned
      (if (Utilities|String|StartsWith _returnvalue_2 "/camera/")
        (Utilities|IsValid (Variables|Default|GetCameraSequenceTrack)
          (:Is%20Valid
            (bind _value (Class|OSCManager|GetFloat Message))
            (switch string (.RightS (Utilities|String|Split _returnvalue_2 "/" "IgnoreCase" "FromEnd"))
              (:position
                (bind _output_get (Variables|Default|SetPosTarget (+ _value (Variables|Default|GetActiveCameraId)))))
              (:id
                (bind _output_get_2 (Variables|Default|SetActiveCameraId (Math|Conversions|ToInteger(Byte) (Class|KismetMathLibrary|Round64 (Math|Float|Max(Float) (- _value 1.0) 0.0)))))
                (bind _returnvalue_3 (Class|OSCManager|GetOSCMessageAddress Message))
                (Class|OSCManager|GetOSCAddressFullPath _returnvalue_3)
                (Development|PrintString (Utilities|String|ToString(Integer) _output_get_2))))))))))

(event Custom|OnSharedServerReady
  (params (OSC%20Server%20Instance :type OSC%20Server%20Object%20Reference))
  (Development|PrintString "Shared OSC server is ready...")
  (Utilities|FlowControl|Sequence
    (:then_0
      (Utilities|IsValid OSC%20Server%20Instance
        (:Is%20Valid
          ;[0 0 0] Setup event
          (EventDispatchers|BindEventtoOnOscMessageReceived OSC%20Server%20Instance (delegate Custom|OnOSCMessageReceived)))
        (:Is%20Not%20Valid
          (Development|PrintString "Server was not valid..."))))))

(event EventTick
  (params (DeltaSeconds :type Float%20%28single-precision%29))
  (Utilities|FlowControl|Sequence
    (:then_0
      (bind _output_get (Variables|Default|SetPosSmoothed (Math|Float|Lerp (Variables|Default|GetPosSmoothed) (Variables|Default|GetPosTarget) (* DeltaSeconds 3.0))))
      (Components|Timeline|SetPlaybackPosition (Variables|/Script/LevelSequence.LevelSequenceActor|GetSequencePlayer (Variables|Default|GetCameraSequenceTrack)) (Utilities|Struct|MakeMovieSceneSequencePlaybackParams "(FrameNumber=(Value=0),SubFrame=0.000000)" _output_get "" "Time" "Jump" false)))))

(event EventBeginPlay
  (Utilities|FlowControl|Sequence
    (:then_0
      ;[0 0 0] Create shared server if it isn't
      (bind _returnvalue (Actor|GetActorOfClass "/Game/IMOGEN26/Blueprints/BP_SharedOscServer.BP_SharedOscServer_C"))
      (Utilities|IsValid _returnvalue
        (:Is%20Not%20Valid
          (Game|SpawnActorfromClass "/Game/IMOGEN26/Blueprints/BP_SharedOscServer.BP_SharedOscServer_C" (Math|Transform|MakeTransform "0, 0, 0") "Undefined" "MultiplyWithRoot" 0 0)
          (Development|PrintString "Auto-Created shared OSC server setup."))))))

(fn ConstructionScript)