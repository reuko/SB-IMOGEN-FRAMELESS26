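; BP_SharedOscServer is an actor that hosts one shared OSC server for the level's OSC-driven Niagara and camera controllers.
; On BeginPlay it creates a listening OSC server named AIMOGEN on port 10000 across all interfaces and stores it.
; It then finds every BP_OscNiagaraController and BP_OscCameraController and passes each the instance through OnSharedServerReady, so they share a single server.
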(event EventBeginPlay
  (Utilities|FlowControl|Sequence
    (:then_0
      ;[0 0 0] Server init
      (bind _returnvalue (Class|OSCManager|CreateOSCServer "0.0.0.0" 10000 false true "AIMOGEN" 0))
      (bind _output_get (Variables|Default|SetOSC%20Server%20Instance _returnvalue))
      (Development|PrintString (Utilities|String|Append "OSC initialized: " (Utilities|GetDisplayName _output_get))))
    (:then_1
      ;[0 0 0] Initialize instances of OSC to Niagara BP
      (bind _outactors (Actor|GetAllActorsOfClass "/Game/IMOGEN26/Blueprints/BP_OscNiagaraController.BP_OscNiagaraController_C"))
      (for _array_element _outactors
        (Default|OnSharedServerReady _array_element (Variables|Default|GetOSC%20Server%20Instance))))
    (:then_2
      ;[0 0 0] Initialize instances of OSC to Niagara BP
      (bind _outactors_2 (Actor|GetAllActorsOfClass "/Game/IMOGEN26/Blueprints/BP_OscCameraController.BP_OscCameraController_C"))
      (for _array_element_2 _outactors_2
        (Default|OnSharedServerReady _array_element_2 (Variables|Default|GetOSC%20Server%20Instance))))))

(fn ConstructionScript)