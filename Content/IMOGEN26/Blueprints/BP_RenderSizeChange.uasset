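; BP_RenderSizeChange is a debug control for changing render resolution scale at runtime from the keyboard.
; Holding 1 raises the scale over time and Shift+1 lowers it, using key-state flags polled on Tick.
; The clamped scale drives an r.ScreenPercentage console command string, and a screen message shows the resulting size computed from the user-settings resolution.
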(event EventBeginPlay
  (Development|PrintString "Set resolution scale with 1 / Shift 1"))

(event EventTick
  (params (DeltaSeconds :type Float%20%28single-precision%29))
  (if (Variables|Default|GetIsPressed)
    (Development|ExecuteConsoleCommand (Utilities|String|Append "r.ScreenPercentage " (Utilities|String|ToString(Float) (* (Math|Float|Clamp(Float) (+ (Variables|Default|GetResScaleNrm) (* DeltaSeconds (Math|Float|SelectFloat -1.0 1.0 (Variables|Default|GetShiftPressed)))) 0.05 2.0) 1e+02))) 0)
    (bind _returnvalue (Settings|GetGameUserSettings))
    (Variables|Default|SetResScaleNrm (Math|Float|Clamp(Float) (+ (Variables|Default|GetResScaleNrm) (* DeltaSeconds (Math|Float|SelectFloat -1.0 1.0 (Variables|Default|GetShiftPressed)))) 0.05 2.0))
    (Development|PrintString (Utilities|String|Append "Res: " (Utilities|String|ToString(Integer) (Math|Float|Round (* (Math|Float|Clamp(Float) (+ (Variables|Default|GetResScaleNrm) (* DeltaSeconds (Math|Float|SelectFloat -1.0 1.0 (Variables|Default|GetShiftPressed)))) 0.05 2.0) (.x (Class|GameUserSettings|GetScreenResolution _returnvalue))))) "x" (Utilities|String|ToString(Integer) (Math|Float|Round (* (Math|Float|Clamp(Float) (+ (Variables|Default|GetResScaleNrm) (* DeltaSeconds (Math|Float|SelectFloat -1.0 1.0 (Variables|Default|GetShiftPressed)))) 0.05 2.0) (.y (Class|GameUserSettings|GetScreenResolution _returnvalue))))) " (" (Utilities|String|ToString(Float) (Math|Float|Clamp(Float) (+ (Variables|Default|GetResScaleNrm) (* DeltaSeconds (Math|Float|SelectFloat -1.0 1.0 (Variables|Default|GetShiftPressed)))) 0.05 2.0)) "x)"))))

(event Input|KeyboardEvents|1
  (params (Key :type Key%20Structure :default "None"))
  (:Pressed
    (Variables|Default|SetIsPressed true))
  (:Released
    (Variables|Default|SetIsPressed false)))

(event Input|KeyboardEvents|LeftShift
  (params (Key :type Key%20Structure :default "None"))
  (:Pressed
    (Variables|Default|SetShiftPressed true))
  (:Released
    (Variables|Default|SetShiftPressed false)))

(fn ConstructionScript)