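; Control actor that drives the second attractor of a referenced Niagara system actor's particle effect.
; Its world location, relative to that actor's root, becomes the attractor's position offset, so moving this actor moves the attractor.
; It also pushes its own strength, radius, mask falloff, noise, vortex and particle scale values into the Niagara user variables.
; The same update runs in the Construction Script and every Tick, covering editor-time placement and runtime changes.
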(event EventBeginPlay)

(event Collision|EventActorBeginOverlap
  (params (OtherActor :type Actor%20Object%20Reference)))

(event EventTick
  (params (DeltaSeconds :type Float%20%28single-precision%29))
  (bind _niagara_system (Variables|Default|GetNiagara%20System))
  (bind _niagaracomponent (Variables|/Script/Niagara.NiagaraActor|GetNiagaraComponent _niagara_system))
  (Niagara|SetNiagaraVariable(Vector3) _niagaracomponent "Attractor02_PositionOffset" (- (Transformation|GetActorLocation) (Transformation|GetWorldLocation (Variables|/Script/Engine.Actor|GetRootComponent _niagara_system))))
  (Niagara|SetNiagaraVariable(Float) _niagaracomponent "Attractor02_Strength" (Variables|Default|GetAttractor02%20Strength))
  (Niagara|SetNiagaraVariable(Float) _niagaracomponent "Attractor02_Mask_Falloff" (Variables|Default|GetAttractor02%20Mask%20Falloff))
  (Niagara|SetNiagaraVariable(Float) _niagaracomponent "Attractor02_Radius" (Variables|Default|GetAttractor02%20Radius))
  (Niagara|SetNiagaraVariable(Float) _niagaracomponent "Attractor02_Noise_Str" (Variables|Default|GetAttractor02%20Noise%20Strength))
  (Niagara|SetNiagaraVariable(Float) _niagaracomponent "Attractor02_Vortex_Str" (Variables|Default|GetAttractor02%20Vortex%20Strength))
  (Niagara|SetNiagaraVariable(Float) _niagaracomponent "Attractor02_PScale" (Variables|Default|GetAttractor02%20PScale)))

(fn ConstructionScript
  (bind _niagara_system (Variables|Default|GetNiagara%20System))
  (bind _niagaracomponent (Variables|/Script/Niagara.NiagaraActor|GetNiagaraComponent _niagara_system))
  (Niagara|SetNiagaraVariable(Vector3) _niagaracomponent "Attractor02_PositionOffset" (- (Transformation|GetActorLocation) (Transformation|GetWorldLocation (Variables|/Script/Engine.Actor|GetRootComponent _niagara_system))))
  (Niagara|SetNiagaraVariable(Float) _niagaracomponent "Attractor02_Strength" (Variables|Default|GetAttractor02%20Strength))
  (Niagara|SetNiagaraVariable(Float) _niagaracomponent "Attractor02_Mask_Falloff" (Variables|Default|GetAttractor02%20Mask%20Falloff))
  (Niagara|SetNiagaraVariable(Float) _niagaracomponent "Attractor02_Radius" (Variables|Default|GetAttractor02%20Radius))
  (Niagara|SetNiagaraVariable(Float) _niagaracomponent "Attractor02_Noise_Str" (Variables|Default|GetAttractor02%20Noise%20Strength))
  (Niagara|SetNiagaraVariable(Float) _niagaracomponent "Attractor02_Vortex_Str" (Variables|Default|GetAttractor02%20Vortex%20Strength))
  (Niagara|SetNiagaraVariable(Float) _niagaracomponent "Attractor02_PScale" (Variables|Default|GetAttractor02%20PScale)))