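; Control actor that drives the first attractor of a referenced Niagara system actor from its own placement and exposed values.
; It sends its location relative to that system's root as a position offset, along with strength, mask falloff, radius, noise, vortex and particle scale parameters.
; The same parameter push runs in the construction script and every Tick, so the effect updates both during editing and at runtime.
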(event EventBeginPlay)

(event Collision|EventActorBeginOverlap
  (params (OtherActor :type Actor%20Object%20Reference)))

(event EventTick
  (params (DeltaSeconds :type Float%20%28single-precision%29))
  (bind _niagara_system (Variables|Default|GetNiagara%20System))
  (bind _niagaracomponent (Variables|/Script/Niagara.NiagaraActor|GetNiagaraComponent _niagara_system))
  (Niagara|SetNiagaraVariable(Vector3) _niagaracomponent "Attractor01_PositionOffset" (- (Transformation|GetActorLocation) (Transformation|GetWorldLocation (Variables|/Script/Engine.Actor|GetRootComponent _niagara_system))))
  (Niagara|SetNiagaraVariable(Float) _niagaracomponent "Attractor01_Strength" (Variables|Default|GetAttractor01%20Strength))
  (Niagara|SetNiagaraVariable(Float) _niagaracomponent "Attractor01_Mask_Falloff" (Variables|Default|GetAttractor01%20Mask%20Falloff))
  (Niagara|SetNiagaraVariable(Float) _niagaracomponent "Attractor01_Radius" (Variables|Default|GetAttractor01%20Radius))
  (Niagara|SetNiagaraVariable(Float) _niagaracomponent "Attractor01_Noise_Str" (Variables|Default|GetAttractor01%20Noise%20Strength))
  (Niagara|SetNiagaraVariable(Float) _niagaracomponent "Attractor01_Vortex_Str" (Variables|Default|GetAttractor01%20Vortex%20Strength))
  (Niagara|SetNiagaraVariable(Float) _niagaracomponent "Attractor01_PScale" (Variables|Default|GetAttractor01%20PScale)))

(fn ConstructionScript
  (bind _niagara_system (Variables|Default|GetNiagara%20System))
  (bind _niagaracomponent (Variables|/Script/Niagara.NiagaraActor|GetNiagaraComponent _niagara_system))
  (Niagara|SetNiagaraVariable(Vector3) _niagaracomponent "Attractor01_PositionOffset" (- (Transformation|GetActorLocation) (Transformation|GetWorldLocation (Variables|/Script/Engine.Actor|GetRootComponent _niagara_system))))
  (Niagara|SetNiagaraVariable(Float) _niagaracomponent "Attractor01_Strength" (Variables|Default|GetAttractor01%20Strength))
  (Niagara|SetNiagaraVariable(Float) _niagaracomponent "Attractor01_Mask_Falloff" (Variables|Default|GetAttractor01%20Mask%20Falloff))
  (Niagara|SetNiagaraVariable(Float) _niagaracomponent "Attractor01_Radius" (Variables|Default|GetAttractor01%20Radius))
  (Niagara|SetNiagaraVariable(Float) _niagaracomponent "Attractor01_Noise_Str" (Variables|Default|GetAttractor01%20Noise%20Strength))
  (Niagara|SetNiagaraVariable(Float) _niagaracomponent "Attractor01_Vortex_Str" (Variables|Default|GetAttractor01%20Vortex%20Strength))
  (Niagara|SetNiagaraVariable(Float) _niagaracomponent "Attractor01_PScale" (Variables|Default|GetAttractor01%20PScale)))